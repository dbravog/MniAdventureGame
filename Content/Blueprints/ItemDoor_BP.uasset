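; ItemDoor_BP is a usable door that swings open and closed when used.
; OnUse flips the IsOpen flag and calls ChangeDoorStatus, which plays the Door_TL timeline from the start to open or reverses it from the end to close.
; The timeline track drives the yaw of the Scene component's relative rotation.
; The construction script sizes the Collision box to the static mesh's bounds.
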(event `ChangeDoorStatus`
  (if (`self.bIsOpen`)
    (bind (_direction _track) (`Timeline|Door_TL` :!via `PlayFromStart` :!label _label)
      (:`Update`
        (`SceneComponent.K2_SetRelativeRotation` (`self.Scene`) (`KismetMathLibrary.MakeRotator` 0.0 0.0 _track) false false)))
    (else
      (goto _label :!via `ReverseFromEnd`))))

(fn `OnUse`
  (set `self.bIsOpen` (not (`self.bIsOpen`)))
  (`self.ChangeDoorStatus`))

(fn `UserConstructionScript`
  (`parent.UserConstructionScript`)
  (`BoxComponent.SetBoxExtent` (`self.Collision`) (`.BoxExtent` (`KismetSystemLibrary.GetComponentBounds` (`self.StaticMesh`))) true))
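; Player Blueprint that identifies which of three named cubes the player is looking at when Use is pressed.
; The input fires a Visibility line trace, drawn persistently for debugging, between two points requested from the Get Location helper.
; That helper's graph holds a math expression offsetting actor location along the control rotation's forward vector by a magnitude.
; The hit actor's display name selects a printed message.
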(event `InputAction|Use`
  (params (Key :type "Key Structure"))
  (:`Pressed`
    (bind (_outhit _returnvalue) (`KismetSystemLibrary.LineTraceSingle` :`Start` (`self.Get Location` 4.0) :`End` (`self.Get Location` 400.0) :`TraceChannel` "TraceTypeQuery1" :`DrawDebugType` "Persistent"))
    (if _returnvalue
      (switch `string` (`KismetSystemLibrary.GetDisplayName` (`.HitActor` (`GameplayStatics.BreakHitResult` _outhit)))
        (:`Cubo1`
          (`KismetSystemLibrary.PrintString` "Es el cubo1" true true (struct :`R` 1.0 :`G` 0.027617 :`B` 0.770973 :`A` 1.0)))
        (:`Cubo2`
          (`KismetSystemLibrary.PrintString` "Es el cubo2" true true (struct :`R` 1.0 :`G` 0.027617 :`B` 0.770973 :`A` 1.0)))
        (:`Cubo3`
          (`KismetSystemLibrary.PrintString` "Es el cubo3" true true (struct :`R` 1.0 :`G` 0.027617 :`B` 0.770973 :`A` 1.0)))))))

(fn `UserConstructionScript`)